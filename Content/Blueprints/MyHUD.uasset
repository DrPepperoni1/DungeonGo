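; MyHUD is a HUD Blueprint that switches the game between main menu, character creation, game and fight screens.
; BeginPlay creates and displays the main menu, and each Show event clears all widgets before adding its own screen to the viewport.
; Main menu, game and fight widgets are cached and reused when valid, while character creation builds a fresh widget on every call.
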(event Custom|ShowCreateCharacter
  (Viewport|RemoveAllWidgets)
  (bind _returnvalue (UserInterface|CreateWidget "/Game/Blueprints/CreateCharacter/CreateWidget.CreateWidget_C" (Game|GetPlayerController 0)))
  (bind _output_get (Variables|Default|SetCreateUI _returnvalue))
  (UserInterface|Viewport|AddtoViewport _output_get 0))

(event Custom|ShowGameView
  (Viewport|RemoveAllWidgets)
  (Utilities|IsValid (Variables|Default|GetGameView)
    (:Is%20Valid
      (UserInterface|Viewport|AddtoViewport (Variables|Default|GetGameView) 0))
    (:Is%20Not%20Valid
      (bind _returnvalue (UserInterface|CreateWidget "/Game/Blueprints/GameView/GameViewWidget.GameViewWidget_C" (Game|GetPlayerController 0)))
      (bind _output_get (Variables|Default|SetGameView _returnvalue))
      (UserInterface|Viewport|AddtoViewport _output_get 0))))

(event Custom|ShowMainMenu
  (Viewport|RemoveAllWidgets)
  (Utilities|IsValid (Variables|Default|GetMAINUI)
    (:Is%20Valid
      (UserInterface|Viewport|AddtoViewport (Variables|Default|GetMAINUI) 0))
    (:Is%20Not%20Valid
      (bind _returnvalue (UserInterface|CreateWidget "/Game/Blueprints/MainMenu/MainMenuWidget.MainMenuWidget_C" (Game|GetPlayerController 0)))
      (bind _output_get (Variables|Default|SetMAINUI _returnvalue))
      (UserInterface|Viewport|AddtoViewport _output_get 0))))

(event Custom|ShowFightView
  (Viewport|RemoveAllWidgets)
  (Utilities|IsValid (Variables|Default|GetFightView)
    (:Is%20Valid
      (UserInterface|Viewport|AddtoViewport (Variables|Default|GetFightView) 0))
    (:Is%20Not%20Valid
      (bind _returnvalue (UserInterface|CreateWidget "/Game/Blueprints/FightView/FightWidget.FightWidget_C" (Game|GetPlayerController 0)))
      (bind _output_get (Variables|Default|SetFightView _returnvalue))
      (UserInterface|Viewport|AddtoViewport _output_get 0))))

(event EventBeginPlay
  (bind _returnvalue (UserInterface|CreateWidget "/Game/Blueprints/MainMenu/MainMenuWidget.MainMenuWidget_C" (Game|GetPlayerController 0)))
  (bind _output_get (Variables|Default|SetMAINUI _returnvalue))
  (UserInterface|Viewport|AddtoViewport _output_get 0))

(fn ConstructionScript)